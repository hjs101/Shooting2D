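; BP_Coding is a practice Blueprint for basic scripting concepts, with sections commented in Korean for loops, conditionals, and data types and variables.
; On BeginPlay, a for loop adds 1 through 10 into AddNum and prints the total.
; The other exercises are disconnected and never run: a cycling switch on ChooseIndex, an IsGood branch, variable prints, empty loops and a SetActorLocation call.
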(event `self.ReceiveBeginPlay`
  ;[1 1 1] 반복문
  (for _index (range 1 11)
    (set `self.AddNum` (+ _index (`self.AddNum`))))
  (`KismetSystemLibrary.PrintString` (`KismetStringLibrary.Conv_IntToString` (`self.AddNum`))))

(event `self.ReceiveTick`
  (params (DeltaSeconds :type "Float (single-precision)")))

(fn `UserConstructionScript`)