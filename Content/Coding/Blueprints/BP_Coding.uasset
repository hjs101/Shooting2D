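; BP_Coding is a scripting practice Blueprint that demonstrates basic concepts through printed output.
; On BeginPlay it passes two variables to the MyAdd function, which returns their sum, and prints the result.
; Disconnected example chains cover variables and types, branching, a switch that cycles an index after a delay, for loops and array ForEach iteration, none of which run.
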(event `self.ReceiveActorBeginOverlap`
  (params (OtherActor :type "Actor Object Reference")))

(event `self.ReceiveTick`
  (params (DeltaSeconds :type "Float (single-precision)")))

(event `self.ReceiveBeginPlay`
  ;[1 1 1] 함수
  (bind _result (`self.MyAdd` (`self.Number`) (`self.AddNum`)))
  (`KismetSystemLibrary.PrintString` (`KismetStringLibrary.Conv_IntToString` _result)))

(fn `MyAdd`
  (params (AddNum1 :type Integer) (AddNum2 :type Integer))
  (returns (Result :type Integer))
  (return (+ AddNum1 AddNum2)))

(fn `UserConstructionScript`)