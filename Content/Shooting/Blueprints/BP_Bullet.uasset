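; BP_Bullet is a projectile actor for the shooting game that destroys enemies it touches.
; Each tick it moves along its forward vector at Speed, scaled by delta time and without sweeping.
; On overlap with a BP_Enemy it destroys the enemy and itself, adds 10 to the Score on BP_ShootingGameModeBase, and plays a 2D explosion sound.
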(event `self.ReceiveTick`
  (params (DeltaSeconds :type "Float (single-precision)"))
  (`self.K2_SetActorLocation` (+ (`self.K2_GetActorLocation`) (* (`self.GetActorForwardVector`) (`self.Speed`) DeltaSeconds))))

(event `self.ReceiveActorBeginOverlap`
  (params (OtherActor :type "Actor Object Reference"))
  (bind _asbp_enemy (cast `/Game/Shooting/Blueprints/BP_Enemy` OtherActor))
  (`self.K2_DestroyActor` _asbp_enemy)
  (`self.K2_DestroyActor`)
  (bind _asbp_shooting_game_mode_base (cast `/Game/Shooting/Blueprints/BP_ShootingGameModeBase` (`GameplayStatics.GetGameMode`)))
  (set `/Game/Shooting/Blueprints/BP_ShootingGameModeBase.Score` (+ (`/Game/Shooting/Blueprints/BP_ShootingGameModeBase.Score` _asbp_shooting_game_mode_base) 10) _asbp_shooting_game_mode_base)
  (`GameplayStatics.PlaySound2D` "/Game/Shooting/Sound/Explosion.Explosion" 1.0 1.0 0.0 null null))

(fn `UserConstructionScript`)