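; BP_Enemy is a shooting-game enemy that flies in a straight line and damages BP_Player on contact.
; At BeginPlay it randomly locks its direction toward the player's position or its own forward vector, favoring the player, then moves unswept each Tick.
; On overlap with the player it calls TakeDamage and destroys itself.
; If the returned value is zero or less, it also destroys the player, pauses, shows WBP_GameOver and plays an explosion.
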(event `self.ReceiveBeginPlay`
  (bind _returnvalue (`GameplayStatics.GetPlayerPawn` 0))
  (if (> (`KismetMathLibrary.RandomIntegerInRange` 0 9) 3)
    (cast `/Game/Shooting/Blueprints/BP_Player` _returnvalue
      (:`then`
        (set `self.MoveVector` (`KismetMathLibrary.Normal` (- (`self.K2_GetActorLocation` _returnvalue) (`self.K2_GetActorLocation`)))))
      (:`CastFailed`
        (set `self.MoveVector` (`self.GetActorForwardVector`) :!label _label)))
    (else
      (goto _label))))

(event `self.ReceiveTick`
  (params (DeltaSeconds :type "Float (single-precision)"))
  (`self.K2_SetActorLocation` (+ (`self.K2_GetActorLocation`) (* (`self.MoveVector`) (`self.Speed`) DeltaSeconds))))

(event `self.ReceiveActorBeginOverlap`
  (params (OtherActor :type "Actor Object Reference"))
  (bind _returnvalue (`GameplayStatics.GetPlayerController` 0))
  ;[1 1 1] 플레이어의 체력 1 소모 및 체력이 0 이하라면 플레이어 파괴
  (bind _asbp_player (cast `/Game/Shooting/Blueprints/BP_Player` OtherActor))
  (bind _newparam (`/Game/Shooting/Blueprints/BP_Player.TakeDamage` _asbp_player))
  (if (<= _newparam 0)
    (`self.K2_DestroyActor` _asbp_player)
    (`GameplayStatics.SetGamePaused` true)
    (bind _returnvalue_2 (`|CreateWidget` "/Game/Shooting/UI/WBP_GameOver.WBP_GameOver_C"))
    (`UserWidget.AddToViewport` _returnvalue_2 0)
    (set `PlayerController.bShowMouseCursor` true _returnvalue)
    (`WidgetBlueprintLibrary.SetInputMode_UIOnlyEx` _returnvalue null)
    (`GameplayStatics.PlaySound2D` "/Game/Shooting/Sound/Audio_Explosion.Audio_Explosion" 1.0 1.0 0.0 null null)
    (`self.K2_DestroyActor`)
    (else
      (`self.K2_DestroyActor`))))

(fn `UserConstructionScript`)