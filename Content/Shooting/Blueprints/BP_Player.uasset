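; Player actor for a shooting game that moves along its up and right axes, fires bullets and tracks HP.
; Tick applies normalized horizontal and vertical input as an unswept, frame-rate-independent location offset.
; Fire input only toggles a flag, which a looping timer polls to spawn BP_Bullet at the Arrow and play a blaster sound.
; TakeDamage decrements HP and pushes the health ratio to the WBP_PlayerHP widget cached at BeginPlay.
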(event `self.ReceiveTick`
  (params (DeltaSeconds :type "Float (single-precision)"))
  ;[1 1 1] 플레이어 이동
  (`self.K2_SetActorLocation` (+ (`self.K2_GetActorLocation`) (* (`KismetMathLibrary.Normal` (+ (* (`self.GetActorUpVector`) (`self.GetInputAxisValue`)) (* (`self.GetActorRightVector`) (`self.GetInputAxisValue`)))) (`self.Speed`) DeltaSeconds))))

(event `InputAction|Fire`
  (params (Key :type "Key Structure"))
  (:`Pressed`
    (set `self.FireState` true))
  (:`Released`
    (set `self.FireState` false)))

(event `self.ReceiveBeginPlay`
  (bind _returnvalue (`GameplayStatics.GetPlayerController` 0))
  (`|ExecutionSequence`
    (:`then_0`
      (`KismetSystemLibrary.K2_SetTimerDelegate` (delegate `FireEvent`) 0.3 true))
    (:`then_1`
      (set `self.HP` (`self.MaxHP`)))
    (:`then_2`
      (set `PlayerController.bShowMouseCursor` false _returnvalue)
      (`WidgetBlueprintLibrary.SetInputMode_GameOnly` _returnvalue))
    (:`then_3`
      (bind _aswbp_player_hp (cast `/Game/Shooting/UI/WBP_PlayerHP` (`WidgetComponent.GetWidget` (`self.WidgetHP`))))
      (set `self.As WBP Player HP` _aswbp_player_hp)
      (`self.UpdateHPUI`))))

(event `FireEvent`
  (if (`self.FireState`)
    (`|SpawnActorFromClass` "/Game/Shooting/Blueprints/BP_Bullet.BP_Bullet_C" (`SceneComponent.K2_GetComponentToWorld` (`self.Arrow`)) "Undefined" "MultiplyWithRoot" null null)
    (`GameplayStatics.PlaySound2D` "/Game/Shooting/Sound/star-wars-blaster.star-wars-blaster" 1.0 1.0 0.0 null null)))

(fn `TakeDamage`
  (returns (NewParam :type Integer))
  (bind _result (`/Engine/EditorBlueprintResources/StandardMacros.DecrementInt` (`self.HP`))
    (:`  `
      (`self.UpdateHPUI`)
      (return _result))))

(fn `UpdateHPUI`
  (set `/Game/Shooting/UI/WBP_PlayerHP.HP` (/ (`self.HP`) (`KismetMathLibrary.Conv_IntToDouble` (`self.MaxHP`))) (`self.As WBP Player HP`)))

(fn `UserConstructionScript`)